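; BP_ZombieGrid is the 25-slot spawner for zombie hands in GMC Challenge 001.
; Between the game mode's start and end events, a looping timer calls Animate Hand at SpawnRate.
; Each call picks a random slot, retrying recursively while that slot has a valid child at index 1, with no guard for a full grid.
; It then spawns and attaches a BP_ZombieHand and increments the game mode's TotalZombies.
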(event `self.ReceiveBeginPlay`
  (bind _asbp_gmcgame_mode_001 (cast `/Game/GMC/Challenges/Challenge_001/Blueprints/BP_GMCGameMode_001` (`GameplayStatics.GetGameMode`)))
  (add `/Game/GMC/Challenges/Challenge_001/Blueprints/BP_GMCGameMode_001.GameStartEvent` _asbp_gmcgame_mode_001 (delegate `GameStartEvent_Event_0`))
  (add `/Game/GMC/Challenges/Challenge_001/Blueprints/BP_GMCGameMode_001.GameEndEvent` _asbp_gmcgame_mode_001 (delegate `GameEndEvent`)))

(event `GameStartEvent_Event_0`
  (`self.Animate Hand`)
  (`KismetSystemLibrary.K2_SetTimer` self "Animate Hand" (`self.SpawnRate`) true))

(event `GameEndEvent`
  (`KismetSystemLibrary.K2_ClearTimer` self "Animate Hand"))

(fn `Animate Hand`
  (locals (MatchFound :type Boolean))
  (bind _output_get (set `self.CurrentHand` (`self.Get Random Index`)))
  (bind _output (`|GetArrayItem` (`self.Get Slot Array`) _output_get))
  (`/Engine/EditorBlueprintResources/StandardMacros.IsValid` (`SceneComponent.GetChildComponent` _output 1)
    (:`Is Valid`
      (`self.Animate Hand`))
    (:`Is Not Valid`
      (`self.Spawn Hand at Location` _output)
      (bind _asbp_gmcgame_mode_001 (cast `/Game/GMC/Challenges/Challenge_001/Blueprints/BP_GMCGameMode_001` (`GameplayStatics.GetGameMode`)))
      (set `/Game/GMC/Challenges/Challenge_001/Blueprints/BP_GMCGameMode_001.TotalZombies` (+ (`/Game/GMC/Challenges/Challenge_001/Blueprints/BP_GMCGameMode_001.TotalZombies` _asbp_gmcgame_mode_001) 1) _asbp_gmcgame_mode_001))))

(fn `Get Random Index`
  (returns (Index :type Integer))
  (return (`KismetMathLibrary.RandomIntegerInRange` 0 (- (`KismetArrayLibrary.Array_Length` (`self.Get Slot Array`)) 1))))

(fn `Get Slot Array`
  (returns (Array :type "Array of SceneComponent Object Reference"))
  (return (`|MakeArray` (`self.Slot01`) (`self.Slot02`) (`self.Slot03`) (`self.Slot04`) (`self.Slot05`) (`self.Slot06`) (`self.Slot07`) (`self.Slot08`) (`self.Slot09`) (`self.Slot10`) (`self.Slot11`) (`self.Slot12`) (`self.Slot13`) (`self.Slot14`) (`self.Slot15`) (`self.Slot16`) (`self.Slot17`) (`self.Slot18`) (`self.Slot19`) (`self.Slot20`) (`self.Slot21`) (`self.Slot22`) (`self.Slot23`) (`self.Slot24`) (`self.Slot25`))))

(fn `Spawn Hand at Location`
  (params (SceneComponent :type "SceneComponent Object Reference"))
  (locals (NewLocalVar_0 :type "Array of SceneComponent Object Reference"))
  (bind _returnvalue (`|SpawnActorFromClass` "/Game/GMC/Challenges/Challenge_001/Blueprints/BP_ZombieHand.BP_ZombieHand_C" (`KismetMathLibrary.Conv_VectorToTransform` (`SceneComponent.K2_GetComponentLocation` SceneComponent)) "Undefined" "OverrideRootScale" self null))
  (`self.K2_AttachToComponent` _returnvalue SceneComponent "None" "SnapToTarget" "SnapToTarget" "KeepRelative" true))

(fn `UserConstructionScript`)