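; BP_ZombieHand is a hittable zombie hand target for GMC Challenge 001.
; BeginPlay caches the hand's currently active montage and creates a dynamic material instance.
; OnHit flashes the emissive parameter for a tenth of a second, jumps the montage to its "End" section, increments ZombiesHit on BP_GMCGameMode_001 and plays a hit sound.
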(event `self.ReceiveBeginPlay`
  (bind _output_get (set `self.ZombieAnimInstance` (`SkeletalMeshComponent.GetAnimInstance` (`self.ZombieHand`))))
  (set `self.ZombieMontage` (`AnimInstance.GetCurrentActiveMontage` _output_get))
  (bind _returnvalue (`PrimitiveComponent.CreateDynamicMaterialInstance` (`self.ZombieHand`) 0 "/Game/GMC/Challenges/Challenge_001/Materials/Props/ZombieHand/MI_ZombieHand.MI_ZombieHand" "ZombieHandMat"))
  (set `self.HandMat` _returnvalue))

(event `OnHit`
  (`self.FlashRed`)
  (`AnimInstance.Montage_JumpToSection` (`self.ZombieAnimInstance`) "End" (`self.ZombieMontage`))
  (bind _asbp_gmcgame_mode_001 (cast `/Game/GMC/Challenges/Challenge_001/Blueprints/BP_GMCGameMode_001` (`GameplayStatics.GetGameMode`)))
  (set `/Game/GMC/Challenges/Challenge_001/Blueprints/BP_GMCGameMode_001.ZombiesHit` (+ (`/Game/GMC/Challenges/Challenge_001/Blueprints/BP_GMCGameMode_001.ZombiesHit` _asbp_gmcgame_mode_001) 1) _asbp_gmcgame_mode_001)
  (`GameplayStatics.PlaySound2D` "/Game/GMC/Challenges/Challenge_001/Audio/SFX/zombie_hit.zombie_hit" 1.0 1.0 0.0 null null))

(event `FlashRed`
  (`MaterialInstanceDynamic.SetScalarParameterValue` (`self.HandMat`) "EmmisiveValue" (`KismetMathLibrary.Lerp` 0.0 0.5 1.0))
  (`KismetSystemLibrary.Delay` 0.1)
  (`MaterialInstanceDynamic.SetScalarParameterValue` (`self.HandMat`) "EmmisiveValue" (`KismetMathLibrary.Lerp` 0.5 0.0 1.0)))

(fn `UserConstructionScript`)