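; BP_GMCHero is the hero character Blueprint, handling the player HUD, weapon hits and victory celebration.
; BeginPlay creates WBP_HUD and adds it to the viewport, while ResetHUD replaces an existing HUD through the same creation path.
; Weapon collision overlaps call OnHit on any BP_ZombieHand.
; Celebrate spawns a camera at VictoryCamPosition, switches the player's view to it and loops a weapon win animation.
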(event `ResetHUD`
  (bind _hud (`self.HUD`))
  (`/Engine/EditorBlueprintResources/StandardMacros.IsValid` _hud
    (:`Is Valid`
      (`Widget.RemoveFromParent` _hud)
      (bind _returnvalue (`|CreateWidget` "/Game/GMC/Challenges/Challenge_001/UI/WBP_HUD.WBP_HUD_C" (`GameplayStatics.GetPlayerController` 0) :!label _label))
      (bind _output_get (set `self.HUD` _returnvalue))
      (`UserWidget.AddToViewport` _output_get 0))))

(event `self.ReceiveBeginPlay`
  (goto _label))

(event `self.WeaponCollision.OnComponentBeginOverlap`
  (params (OverlappedComponent :type "PrimitiveComponent Object Reference") (OtherActor :type "Actor Object Reference") (OtherComp :type "PrimitiveComponent Object Reference") (OtherBodyIndex :type Integer) (bFromSweep :type Boolean) (SweepResult :type "HitResult Structure (by ref)"))
  (if (!= OtherActor self)
    (bind _asbp_zombie_hand (cast `/Game/GMC/Challenges/Challenge_001/Blueprints/BP_ZombieHand` OtherActor))
    (`/Game/GMC/Challenges/Challenge_001/Blueprints/BP_ZombieHand.OnHit` _asbp_zombie_hand)))

(event `Celebrate`
  (bind _returnvalue (`|SpawnActorFromClass` "/Script/Engine.CameraActor" (`SceneComponent.K2_GetComponentToWorld` (`self.VictoryCamPosition`)) "Undefined" "OverrideRootScale" (`GameplayStatics.GetPlayerController` 0) null))
  (`PlayerController.SetViewTargetWithBlend` (`GameplayStatics.GetPlayerController` 0) _returnvalue 0.0 "VTBlend_Linear" 0.0 false)
  (`SkeletalMeshComponent.PlayAnimation` (`self.Mesh`) "/Game/GMC/GlobalAssets/Characters/Animations/Anim_Win_Weapon.Anim_Win_Weapon" true))

(fn `UserConstructionScript`)